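; BP_Target is a shooting target in the multiplayer FPS that tips over when damaged and stands back up after a short delay.
; Any damage while Ready clears the flag and starts a one-shot timer that restores it.
; Tick calls MoveTarget, which eases the root's roll between upright and lying flat with FInterpTo.
; The construction script caches the placed yaw, in a variable misleadingly named Pitch, to preserve facing.
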(event Custom|RestoreTarget
  (Variables|Default|SetReady? true))

(event Game|Damage|EventAnyDamage
  (params (Damage :type Float%20%28single-precision%29) (DamageType :type Damage%20Type%20Object%20Reference) (InstigatedBy :type Controller%20Object%20Reference) (DamageCauser :type Actor%20Object%20Reference))
  (if (Variables|Default|GetReady?)
    (Variables|Default|SetReady? false)
    (Utilities|Time|SetTimerbyEvent (delegate Custom|RestoreTarget) 5.0)))

(event EventTick
  (params (DeltaSeconds :type Float%20%28single-precision%29))
  (Utilities|MoveTarget DeltaSeconds))

(fn ConstructionScript
  (Variables|Default|SetPitch (.yaw (Transformation|GetWorldRotation (Variables|Default|GetDefaultSceneRoot)))))