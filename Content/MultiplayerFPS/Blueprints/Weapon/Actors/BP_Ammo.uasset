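; BP_Ammo is an ammo pickup actor that grants its Type and Count to a character's weapon component via ServerAddAmmo, then destroys itself.
; Pickup triggers through Interact, or on sphere overlap when the character's InteractTrigger is set.
; Outline enables custom depth on the mesh, with a short timer clearing it once calls stop.
; The construction script applies the configured mesh, and MulticastSetCollision toggles the sphere's collision.
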(event OnComponentBeginOverlap(Sphere)
  (params (OverlappedComponent :type Primitive%20Component%20Object%20Reference) (OtherActor :type Actor%20Object%20Reference) (OtherComp :type Primitive%20Component%20Object%20Reference) (OtherBodyIndex :type Integer) (bFromSweep :type Boolean) (SweepResult :type Hit%20Result%20Structure%20%28by%20ref%29))
  ;[1 1 1] Overlap Take Ammo System
  (bind _asbp_character (Utilities|Casting|CastToBP_Character OtherActor))
  (if (Variables|/Game/MultiplayerFPS/Blueprints/Weapon/Components/BPC_WeaponComponent.BPC_WeaponComponent_C|GetInteract/Trigger? (Variables|/Game/MultiplayerFPS/Blueprints/Player/BP_Character.BP_Character_C|GetBPC_WeaponComponent _asbp_character))
    (Default|ServerAddAmmo (Variables|/Game/MultiplayerFPS/Blueprints/Player/BP_Character.BP_Character_C|GetBPC_WeaponComponent _asbp_character) (Variables|Default|GetType) (Variables|Default|GetCount))
    (Actor|DestroyActor)))

(event Custom|StopOutline
  ;[1 1 1] Outline On Look Function ( You can chage it )
  (Rendering|SetRenderCustomDepth (Variables|Default|GetSkeletalMesh) false))

(event Custom|MulticastSetCollision
  (params (Active? :type Boolean))
  ;[1 1 1] Overlap Take Ammo System
  (Collision|SetCollisionEnabled (Variables|Default|GetSphere) (select Active? "QueryAndPhysics" "NoCollision")) ; Off Collision on take
)

(event EventBeginPlay)

(event EventInteract
  (params (Owner :type BP%20Character%20Object%20Reference))
  ;[1 1 1] Interact Event
  (Default|ServerAddAmmo (Variables|/Game/MultiplayerFPS/Blueprints/Player/BP_Character.BP_Character_C|GetBPC_WeaponComponent Owner) (Variables|Default|GetType) (Variables|Default|GetCount))
  (Actor|DestroyActor))

(event EventOutline
  ;[1 1 1] Outline On Look Function ( You can chage it )
  (Rendering|SetRenderCustomDepth (Variables|Default|GetSkeletalMesh) true) ; OutlineObject
  (Utilities|Time|SetTimerbyFunctionName 0 "StopOutline" 0.05))

(fn ConstructionScript
  (Class|SkinnedMeshComponent|SetSkeletalMesh (Variables|Default|GetSkeletalMesh) (Variables|Default|GetSKMesh) true))